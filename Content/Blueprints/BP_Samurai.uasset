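; Samurai duelist Blueprint for a quick-draw duel run by GM_Duel, with timelines that slide its Paper2D sprite into place and lunge it to attack.
; Attack allows one press per round: pressing during Wait shows a cross and locks out input, while Draw finishes the game and lunges.
; The lunge's event track swaps the sprite and reports success to GM_Duel, flagged by player control.
; Defeated and Reset handle losing and restarting.
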(event Custom|SlideIN
  (Components|Timeline|SetPlayRate (Variables|Default|GetSlideInAnim) 2.0)
  (bind _alpha (Timeline|SlideInAnim PlayFromStart)
    (:Update
      (Transformation|SetRelativeLocation (Variables|Default|GetPaperSprite) (Math|Vector|Lerp(Vector) (Variables|Default|GetSlideStartPos) (Variables|Default|GetSpriteDefaultPaos) _alpha) false false)
      (CallFunction|SetCrossVisibility false))))

(event Custom|Attack
  (if (not (Variables|Default|GetPressedDraw))
    (switch Utilities|FlowControl|Switch|SwitchonE_Phase (Variables|/Game/Blueprints/GM_Duel.GM_Duel_C|GetPhase (Variables|Default|GetGameMode))
      (:NewEnumerator1
        (CallFunction|SetCrossVisibility true)
        (Variables|Default|SetPressedDraw true))
      (:NewEnumerator2
        (Variables|Default|SetPressedDraw true)
        (Default|SetGameFinished (Variables|Default|GetGameMode))
        (Components|Timeline|SetPlayRate (Variables|Default|GetAttackAnim) 8.0)
        (bind _alpha (Timeline|AttackAnim Play)
          (:Update
            (Transformation|SetRelativeLocation (Variables|Default|GetPaperSprite) (Math|Vector|Lerp(Vector) (Variables|Default|GetSpriteDefaultPaos) (Variables|/Script/Engine.SceneComponent|GetRelativeLocation (Variables|Default|GetAttackPos)) _alpha) false false))
          (:SwitchSprite
            (Rendering|Components|Sprite|SetSprite (Variables|Default|GetPaperSprite) (Variables|Default|GetAttackingSptire))
            (Default|AttackSuccessfully (Variables|Default|GetGameMode) (Pawn|IsPlayerControlled))))))))

(event Custom|Defeated
  (Rendering|Components|Sprite|SetSprite (Variables|Default|GetPaperSprite) (Variables|Default|GetDefeatedSprite))
  (CallFunction|SetCrossVisibility false))

(event EventBeginPlay
  (bind _asgm_duel (Utilities|Casting|CastToGM_Duel (Game|GetGameMode)))
  (Variables|Default|SetGameMode _asgm_duel)
  (Variables|Default|SetSpriteDefaultPaos (Variables|/Script/Engine.SceneComponent|GetRelativeLocation (Variables|Default|GetPaperSprite)))
  (CallFunction|SlideIN))

(fn ConstructionScript)

(fn SetCrossVisibility
  (params (bNewVisibility :type Boolean))
  (Rendering|SetVisibility (Variables|Default|GetCross) bNewVisibility false))

(fn Reset
  (Rendering|Components|Sprite|SetSprite (Variables|Default|GetPaperSprite) (Variables|Default|GetIdleSprite))
  (Variables|Default|SetPressedDraw false)
  (CallFunction|SlideIN))